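; Game mode Blueprint for a space game that owns the main menu and controls when it is shown.
; On BeginPlay it creates the WG_Main_Menu widget for the first player controller, caches it and shows it.
; Show and close events add or remove the widget while toggling the mouse cursor and switching between UI-only and game-only input.
; The player spawn event is an empty stub.
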(event `self.ReceiveBeginPlay`
  ; when function get called first time
  (bind _returnvalue (`|CreateWidget` "/Game/UI/WG_Main_Menu.WG_Main_Menu_C" (`GameplayStatics.GetPlayerController` 0)))
  (set `self.WG_Main_Menu Ref` _returnvalue)
  (`self.Show main menu`))

(event `Spawn the player`)

(event `Show main menu`
  (bind _returnvalue (`GameplayStatics.GetPlayerController` 0))
  (bind _wg_main_menu_ref (`self.WG_Main_Menu Ref`))
  ; To show main menu
  (set `PlayerController.bShowMouseCursor` true _returnvalue)
  (`WidgetBlueprintLibrary.SetInputMode_UIOnlyEx` _returnvalue _wg_main_menu_ref)
  (`UserWidget.AddToViewport` _wg_main_menu_ref 0))

(event `Close the main menu`
  (bind _returnvalue (`GameplayStatics.GetPlayerController` 0))
  ; To hide the main menu
  (set `PlayerController.bShowMouseCursor` false _returnvalue)
  (`WidgetBlueprintLibrary.SetInputMode_GameOnly` _returnvalue)
  (`Widget.RemoveFromParent` (`self.WG_Main_Menu Ref`)))

(fn `UserConstructionScript`)